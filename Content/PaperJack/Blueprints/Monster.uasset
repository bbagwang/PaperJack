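; Monster is a bee or wasp enemy actor that patrols in a sine wave and knocks the PaperJack player sideways on touch.
; Tick moves it along Y or Z, as set by the left-right or up-down flag, offsetting its location by the change in sine.
; The sign of that delta picks the facing flipbook, with WaspMode choosing the skin.
; On box overlap, relative Y position selects which push vector launches the player.
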(event OnComponentBeginOverlap(Box)
  (params (OverlappedComponent :type Primitive%20Component%20Object%20Reference) (OtherActor :type Actor%20Object%20Reference) (OtherComp :type Primitive%20Component%20Object%20Reference) (OtherBodyIndex :type Integer) (bFromSweep :type Boolean) (SweepResult :type Hit%20Result%20Structure%20%28by%20ref%29))
  (bind _aspaper_jack (Utilities|Casting|CastToPaperJack OtherActor))
  (Math|Float|CompareFloat (- (.y (Transformation|GetWorldLocation (Variables|Default|GetScene))) (.Y (Math|Vector|BreakVector (Transformation|GetWorldLocation (Variables|/Script/Engine.Character|GetCapsuleComponent _aspaper_jack))))) 0.0
    (:>
      (Character|LaunchCharacter _aspaper_jack (Variables|Default|GetRightSidePushVector) true false))
    (:<
      (Character|LaunchCharacter _aspaper_jack (Variables|Default|GetLeftSidePushVector) true false))))

(event Custom|UpDownMovement
  (params (DeltaTime :type Float%20%28single-precision%29))
  (Variables|Default|SetLocation (Transformation|GetWorldLocation (Variables|Default|GetScene)))
  (bind _output_get (Variables|Default|SetDeltaMove (- (Math|Trig|Sin(Radians) (+ (Variables|Default|GetTimeRunner) DeltaTime)) (Math|Trig|Sin(Radians) (Variables|Default|GetTimeRunner)))))
  (bind _output_get_2 (Variables|Default|SetLocation (Math|Vector|MakeVector (.x (Variables|Default|GetLocation)) (.y (Variables|Default|GetLocation)) (+ (.z (Variables|Default|GetLocation)) (* _output_get (Variables|Default|GetMoveSpeed))))))
  (Variables|Default|SetTimeRunner (+ DeltaTime (Variables|Default|GetTimeRunner)))
  (Transformation|SetActorLocation _output_get_2 false false))

(event Custom|LeftRightMovemnet
  (params (DeltaTime :type Float%20%28single-precision%29))
  (Variables|Default|SetLocation (Transformation|GetWorldLocation (Variables|Default|GetScene)))
  (bind _output_get (Variables|Default|SetDeltaMove (- (Math|Trig|Sin(Radians) (+ (Variables|Default|GetTimeRunner) DeltaTime)) (Math|Trig|Sin(Radians) (Variables|Default|GetTimeRunner)))))
  (bind _output_get_2 (Variables|Default|SetLocation (Math|Vector|MakeVector (.x (Variables|Default|GetLocation)) (+ (.y (Variables|Default|GetLocation)) (* _output_get (Variables|Default|GetMoveSpeed))) (.z (Variables|Default|GetLocation)))))
  (Variables|Default|SetTimeRunner (+ DeltaTime (Variables|Default|GetTimeRunner)))
  (Transformation|SetActorLocation _output_get_2 false false))

(event EventBeginPlay)

(event EventTick
  (params (DeltaSeconds :type Float%20%28single-precision%29))
  (Math|Float|CompareFloat (Variables|Default|GetDeltaMove) 0.0
    (:>
      (if (Variables|Default|GetWaspMode)
        (Sprite|SetFlipbook (Variables|Default|GetPaperFlipbook) "/Game/PaperJack/Textures/Monster/wasp_right.Wasp_Right")
        (else
          (Sprite|SetFlipbook (Variables|Default|GetPaperFlipbook) "/Game/PaperJack/Textures/Monster/bee_right.Bee_Right"))))
    (:==
      _)
    (:<
      (if (Variables|Default|GetWaspMode)
        (Sprite|SetFlipbook (Variables|Default|GetPaperFlipbook) "/Game/PaperJack/Textures/Monster/Wasp.Wasp")
        (else
          (Sprite|SetFlipbook (Variables|Default|GetPaperFlipbook) "/Game/PaperJack/Textures/Monster/Bee.Bee")))))
  (if (Variables|Default|GetIsLeftRightBlock)
    (CallFunction|LeftRightMovemnet self DeltaSeconds)
    (elif (Variables|Default|GetIsUpDownBlock)
      (CallFunction|UpDownMovement self DeltaSeconds))))

(fn ConstructionScript
  (if (Variables|Default|GetWaspMode)
    (Sprite|SetFlipbook (Variables|Default|GetPaperFlipbook) "/Game/PaperJack/Textures/Monster/Wasp.Wasp")
    (else
      (Sprite|SetFlipbook (Variables|Default|GetPaperFlipbook) "/Game/PaperJack/Textures/Monster/Bee.Bee"))))