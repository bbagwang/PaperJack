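; Paper2D thorn hazard in PaperJack that periodically becomes dangerous and knocks the player character sideways.
; A looping Tick countdown, split by configurable thresholds, swaps three sprite states and enables HitPos overlap collision and the IsHit flag only during the hit window.
; On overlap during that window, PaperJack is launched with a left or right push vector chosen by its Y position relative to HitPos.
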(event OnComponentBeginOverlap(HitPos)
  (params (OverlappedComponent :type Primitive%20Component%20Object%20Reference) (OtherActor :type Actor%20Object%20Reference) (OtherComp :type Primitive%20Component%20Object%20Reference) (OtherBodyIndex :type Integer) (bFromSweep :type Boolean) (SweepResult :type Hit%20Result%20Structure%20%28by%20ref%29))
  (bind _aspaper_jack (Utilities|Casting|CastToPaperJack OtherActor))
  (if (Variables|Default|GetIsHit)
    (Math|Float|CompareFloat (- (.y (Transformation|GetWorldLocation (Variables|Default|GetHitPos self))) (.Y (Math|Vector|BreakVector (Transformation|GetWorldLocation (Variables|/Script/Engine.Character|GetCapsuleComponent _aspaper_jack))))) 0.0
      (:>
        (Character|LaunchCharacter _aspaper_jack (Variables|Default|GetRightSidePushVector) true false))
      (:<
        (Character|LaunchCharacter _aspaper_jack (Variables|Default|GetLeftSidePushVector) true false)))))

(event EventTick
  (params (DeltaSeconds :type Float%20%28single-precision%29))
  (bind _output_get (Variables|Default|SetTimer (- (Variables|Default|GetTimer) DeltaSeconds)))
  (Math|Float|CompareFloat _output_get (Variables|Default|GetReadyStartTime)
    (:>
      (Rendering|Components|Sprite|SetSprite (Variables|Default|GetThornSprite) "/Game/PaperJack/Textures/Blocks/thorn_03_Sprite.thorn_03_Sprite")
      (Variables|Default|SetIsHit false)
      (Collision|SetCollisionProfileName (Variables|Default|GetHitPos) "NoCollision" :!class /Script/Engine.PrimitiveComponent))
    (:<
      (if (> (Variables|Default|GetTimer) (Variables|Default|GetHitStartTimer))
        (Rendering|Components|Sprite|SetSprite (Variables|Default|GetThornSprite) "/Game/PaperJack/Textures/Blocks/thorn_02_Sprite.thorn_02_Sprite")
        (Variables|Default|SetIsHit false)
        (Collision|SetCollisionProfileName (Variables|Default|GetHitPos) "NoCollision" :!class /Script/Engine.PrimitiveComponent)
        (elif (<= (Variables|Default|GetTimer) (Variables|Default|GetHitEndTimer))
          (Rendering|Components|Sprite|SetSprite (Variables|Default|GetThornSprite) "/Game/PaperJack/Textures/Blocks/thorn_02_Sprite.thorn_02_Sprite")
          (if (<= (Variables|Default|GetTimer) 0.0)
            (Variables|Default|SetTimer (Variables|Default|GetTimerSave))
            (Variables|Default|SetIsHit false)
            (Collision|SetCollisionProfileName (Variables|Default|GetHitPos) "NoCollision" :!class /Script/Engine.PrimitiveComponent)
            (else
              (Collision|SetCollisionProfileName (Variables|Default|GetHitPos) "NoCollision" :!class /Script/Engine.PrimitiveComponent)))
          (else
            (Rendering|Components|Sprite|SetSprite (Variables|Default|GetThornSprite) "/Game/PaperJack/Textures/Blocks/thorn_01_Sprite.thorn_01_Sprite")
            (Variables|Default|SetIsHit true)
            (Collision|SetCollisionProfileName (Variables|Default|GetHitPos) "OverlapAll" :!class /Script/Engine.PrimitiveComponent)))))))

(event EventBeginPlay
  (Variables|Default|SetTimerSave (Variables|Default|GetTimer)))

(fn ConstructionScript)