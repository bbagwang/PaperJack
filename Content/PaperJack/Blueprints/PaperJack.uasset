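; PaperJack is the 2D flipbook player character, with left/right movement, jumping and axis-driven vertical climbing while CanClimb is set.
; Tick picks flipbooks from velocity and facing, using a fall timer to delay the Drop pose, and switches to Climb when climbing.
; It also drives UI: a start overlay fades into a tutorial on input, and IsGameEnd adds the GameEnd widget every tick.
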(event Custom|CloseOverlay
  ;[1 1 1] CloseOverlay
  (bind _fade (Timeline|Fade Play)
    (:Update
      (Appearance|SetColorandOpacity (Variables|Default|GetWidget) (Utilities|Struct|MakeLinearColor _fade _fade _fade _fade) :!class /Script/UMG.UserWidget)
      (Utilities|FlowControl|Delay 2.0)
      (Viewport|RemoveAllWidgets)
      (bind _returnvalue (UserInterface|CreateWidget "/Game/PaperJack/Blueprints/Tutorial.Tutorial_C"))
      (UserInterface|Viewport|AddtoViewport _returnvalue 0))))

(event Custom|UpdateAnimation
  (params (DeltaTime :type Float%20%28single-precision%29))
  (bind _returnvalue (Transformation|GetVelocity))
  (bind (_x _y _z) (Math|Vector|BreakVector _returnvalue))
  ;[1 1 1] Updating Animation by Actor Velocity
  (Math|Float|CompareFloat _z 0.0
    (:>
      (Variables|Default|Setfalling%20timer 0.0)
      (if (Variables|Default|GetIsRight)
        (Sprite|SetFlipbook (Variables|Default|GetSprite) "/Game/PaperJack/Textures/JACK_Sprite/Jump_Left.Jump_Left")
        (else
          (Sprite|SetFlipbook (Variables|Default|GetSprite) "/Game/PaperJack/Textures/JACK_Sprite/Jump.Jump"))))
    (:==
      (Math|Float|CompareFloat _y 0.0
        (:>
          (Sprite|SetFlipbook (Variables|Default|GetSprite) "/Game/PaperJack/Textures/JACK_Sprite/Run.Run"))
        (:==
          (Sprite|SetFlipbook (Variables|Default|GetSprite) "/Game/PaperJack/Textures/JACK_Sprite/Stand.Stand"))
        (:<
          (Sprite|SetFlipbook (Variables|Default|GetSprite) "/Game/PaperJack/Textures/JACK_Sprite/Run_Left.Run_Left"))))
    (:<
      (bind _output_get (Variables|Default|Setfalling%20timer (+ (Variables|Default|Getfalling%20timer) DeltaTime)))
      (if (>= _output_get (Variables|Default|Getfalling%20start%20point))
        (Sprite|SetFlipbook (Variables|Default|GetSprite) "/Game/PaperJack/Textures/JACK_Sprite/Drop.Drop")
        (elif (Variables|Default|GetIsRight)
          (Sprite|SetFlipbook (Variables|Default|GetSprite) "/Game/PaperJack/Textures/JACK_Sprite/Jump_Left.Jump_Left")
          (else
            (Sprite|SetFlipbook (Variables|Default|GetSprite) "/Game/PaperJack/Textures/JACK_Sprite/Jump.Jump")))))))

(event Custom|Falling%20Check
  (params (DeltaTime :type Float%20%28single-precision%29))
  ;[1 1 1] Updating Animation by Actor Velocity
  (if (< (.Z (Math|Vector|BreakVector (Variables|/Script/Engine.MovementComponent|GetVelocity (Variables|Character|GetCharacterMovement)))) 0.0)
    (bind _output_get (Variables|Default|Setfalling%20timer (+ DeltaTime (Variables|Default|Getfalling%20timer))))
    (Variables|Default|SetIsFalling (>= _output_get (Variables|Default|Getfalling%20start%20point)))
    (else
      (Variables|Default|Setfalling%20timer 0.0)
      (Variables|Default|SetIsFalling false))))

(event EventTick
  (params (DeltaSeconds :type Float%20%28single-precision%29))
  ;[1 1 1] Tick
  (if (Variables|Default|GetIsGameEnd)
    (Variables|/Script/Engine.PlayerController|SetbShowMouseCursor (Game|GetPlayerController 0) true)
    (bind _returnvalue (UserInterface|CreateWidget "/Game/PaperJack/Blueprints/GameEnd.GameEnd_C"))
    (UserInterface|Viewport|AddtoViewport _returnvalue 0)
    (elif (Variables|Default|GetCanClimb)
      (Utilities|FlowControl|DoOnce false :!label _label
        (:Completed
          (Components|Movement|StopMovementImmediately (Variables|Character|GetCharacterMovement))
          (Sprite|SetFlipbook (Variables|Default|GetSprite) "/Game/PaperJack/Textures/JACK_Sprite/Climb.Climb")))
      (else
        (Utilities|FlowControl|Sequence
          (:then_0
            (goto _label Reset))
          (:then_1
            (CallFunction|UpdateAnimation DeltaSeconds)))))))

(event EventBeginPlay
  (Variables|/Script/Engine.PlayerController|SetbShowMouseCursor (Game|GetPlayerController 0) false)
  (Class|ActorComponent|SetIsReplicated (Variables|Default|GetSprite) true)
  (bind _returnvalue (UserInterface|CreateWidget "/Game/PaperJack/Blueprints/GameStart.GameStart_C"))
  (bind _output_get (Variables|Default|SetWidget _returnvalue))
  (UserInterface|Viewport|AddtoViewport _output_get 0))

(event Input|ActionEvents|InputActionJump
  (params (Key :type Key%20Structure))
  ;[1 1 1] Movement
  (:Pressed
    (if (not (Variables|Default|GetIsGameEnd))
      (if (Variables|Default|GetCanClimb)
        (Variables|Default|SetIsClimbJump true)
        (else
          (Variables|Default|SetIsClimbJump false)
          (Character|Jump)))))
  (:Released
    (if (not (Variables|Default|GetIsGameEnd))
      (Character|StopJumping))))

(event Input|ActionEvents|InputActionGameStart
  (params (Key :type Key%20Structure))
  (:Pressed
    (Utilities|FlowControl|DoOnce false
      (:Completed
        (Variables|Default|SetIsGameStart true)
        (CallFunction|CloseOverlay)))))

(event Input|AxisEvents|InputAxisMoveLeftRight
  (params (AxisValue :type Float%20%28single-precision%29))
  ;[1 1 1] Movement
  (if (not (Variables|Default|GetIsGameEnd))
    (Math|Float|CompareFloat AxisValue 0.0
      (:>
        (Variables|Default|SetIsRight true)
        (Pawn|Input|AddMovementInput "0,-1.000000, 0" (Variables|Default|GetMoveSpeed) false))
      (:<
        (Variables|Default|SetIsRight false)
        (Pawn|Input|AddMovementInput "0,1.000000, 0" (Variables|Default|GetMoveSpeed) false)))))

(event Input|AxisEvents|InputAxisClimb
  (params (AxisValue :type Float%20%28single-precision%29))
  (bind _returnvalue (Transformation|GetActorLocation))
  (if (Variables|Default|GetCanClimb)
    (Transformation|SetActorLocation (Math|Vector|MakeVector (.x _returnvalue) (.y _returnvalue) (+ (.z _returnvalue) (* AxisValue (Variables|Default|GetClimbSpeed)))) false false)))

(fn ConstructionScript)