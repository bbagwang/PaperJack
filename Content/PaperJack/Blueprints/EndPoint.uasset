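; EndPoint is the level goal trigger for PaperJack that ends the game when its box is overlapped.
; On overlap it shows the mouse cursor, flags the player's PaperJack pawn as game-ended, hides its sphere and switches Jack's flipbook to the End animation.
; It then creates the GameEnd widget and adds it to the viewport.
; The overlapping actor is not checked; the player pawn is fetched directly.
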(event OnComponentBeginOverlap(Box)
  (params (OverlappedComponent :type Primitive%20Component%20Object%20Reference) (OtherActor :type Actor%20Object%20Reference) (OtherComp :type Primitive%20Component%20Object%20Reference) (OtherBodyIndex :type Integer) (bFromSweep :type Boolean) (SweepResult :type Hit%20Result%20Structure%20%28by%20ref%29))
  (Variables|/Script/Engine.PlayerController|SetbShowMouseCursor (Game|GetPlayerController 0) true)
  (bind _aspaper_jack (Utilities|Casting|CastToPaperJack (Game|Player|GetPlayerPawn 0)))
  (Variables|/Game/PaperJack/Blueprints/PaperJack.PaperJack_C|SetIsGameEnd _aspaper_jack true)
  (Development|SetHiddeninGame (Variables|Default|GetSphere) true false)
  (Sprite|SetFlipbook (Variables|/Script/Paper2D.PaperCharacter|GetSprite _aspaper_jack) "/Game/PaperJack/Textures/JACK_Sprite/End.End")
  (bind _returnvalue (UserInterface|CreateWidget "/Game/PaperJack/Blueprints/GameEnd.GameEnd_C" (Game|GetPlayerController 0)))
  (UserInterface|Viewport|AddtoViewport _returnvalue 0))

(fn ConstructionScript)