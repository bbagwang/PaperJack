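; Leaf platform for PaperJack that can sway left-right or up-down and optionally vanish on a timer after being touched.
; Tick moves it by sine deltas, with left-right taking priority over up-down.
; In hide mode, an Upper overlap starts a countdown with material swaps, then the leaf loses visibility and collision until HideTime runs out and resets it.
; Lower overlap disables Upper and Blocker collision, allowing passage from below.
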(event OnComponentBeginOverlap(Lower)
  (params (OverlappedComponent :type Primitive%20Component%20Object%20Reference) (OtherActor :type Actor%20Object%20Reference) (OtherComp :type Primitive%20Component%20Object%20Reference) (OtherBodyIndex :type Integer) (bFromSweep :type Boolean) (SweepResult :type Hit%20Result%20Structure%20%28by%20ref%29))
  (Utilities|Casting|CastToPaperJack OtherActor)
  (Collision|SetCollisionEnabled (Variables|Default|GetUpper) "NoCollision")
  (Collision|SetCollisionProfileName (Variables|Default|GetBlocker) "NoCollision" :!class /Script/Engine.PrimitiveComponent))

(event OnComponentEndOverlap(Lower)
  (params (OverlappedComponent :type Primitive%20Component%20Object%20Reference) (OtherActor :type Actor%20Object%20Reference) (OtherComp :type Primitive%20Component%20Object%20Reference) (OtherBodyIndex :type Integer))
  (Utilities|Casting|CastToPaperJack OtherActor)
  (Collision|SetCollisionEnabled (Variables|Default|GetUpper) "QueryAndPhysics")
  (Collision|SetCollisionProfileName (Variables|Default|GetBlocker) "BlockAll" :!class /Script/Engine.PrimitiveComponent))

(event OnComponentBeginOverlap(Upper)
  (params (OverlappedComponent :type Primitive%20Component%20Object%20Reference) (OtherActor :type Actor%20Object%20Reference) (OtherComp :type Primitive%20Component%20Object%20Reference) (OtherBodyIndex :type Integer) (bFromSweep :type Boolean) (SweepResult :type Hit%20Result%20Structure%20%28by%20ref%29))
  (Utilities|Casting|CastToPaperJack OtherActor)
  (Variables|Default|SetIsStart true))

(event Custom|Hide
  (params (DeltaTime :type Float%20%28single-precision%29))
  (Development|SetHiddeninGame (Variables|Default|GetPlane) true false)
  (Collision|SetCollisionEnabled (Variables|Default|GetUpper) "NoCollision")
  (bind _output_get (Variables|Default|SetHideTime (- (Variables|Default|GetHideTime) DeltaTime)))
  (if (<= _output_get 0.0)
    (CallFunction|StopHide)))

(event Custom|StopHide
  (Development|SetHiddeninGame (Variables|Default|GetPlane) false false)
  (Collision|SetCollisionEnabled (Variables|Default|GetUpper) "QueryOnly")
  (Collision|SetCollisionEnabled (Variables|Default|GetLower) "QueryOnly")
  (Collision|SetCollisionEnabled (Variables|Default|GetBlocker) "PhysicsOnly")
  (Collision|SetCollisionProfileName (Variables|Default|GetBlocker) "BlockAll" :!class /Script/Engine.PrimitiveComponent)
  (Variables|Default|SetHideTime (Variables|Default|GetSavedHideTime))
  (Variables|Default|SetLifeTime (Variables|Default|GetSavedLifeTime))
  (Variables|Default|SetIsStart false))

(event Custom|UpDownMovement
  (params (DeltaTime :type Float%20%28single-precision%29))
  (Variables|Default|SetLocation (Transformation|GetWorldLocation (Variables|Default|GetScene)))
  (bind _output_get (Variables|Default|SetDeltaMove (- (Math|Trig|Sin(Radians) (+ (Variables|Default|GetTimeRunner) DeltaTime)) (Math|Trig|Sin(Radians) (Variables|Default|GetTimeRunner)))))
  (bind _output_get_2 (Variables|Default|SetLocation (Math|Vector|MakeVector (.x (Variables|Default|GetLocation)) (.y (Variables|Default|GetLocation)) (+ (.z (Variables|Default|GetLocation)) (* _output_get (Variables|Default|GetMoveSpeed))))))
  (Variables|Default|SetTimeRunner (+ DeltaTime (Variables|Default|GetTimeRunner)))
  (Transformation|SetActorLocation _output_get_2 false false))

(event Custom|LeftRightMovemnet
  (params (DeltaTime :type Float%20%28single-precision%29))
  (Variables|Default|SetLocation (Transformation|GetWorldLocation (Variables|Default|GetScene)))
  (bind _output_get (Variables|Default|SetDeltaMove (- (Math|Trig|Sin(Radians) (+ (Variables|Default|GetTimeRunner) DeltaTime)) (Math|Trig|Sin(Radians) (Variables|Default|GetTimeRunner)))))
  (bind _output_get_2 (Variables|Default|SetLocation (Math|Vector|MakeVector (.x (Variables|Default|GetLocation)) (+ (.y (Variables|Default|GetLocation)) (* _output_get (Variables|Default|GetMoveSpeed))) (.z (Variables|Default|GetLocation)))))
  (Variables|Default|SetTimeRunner (+ DeltaTime (Variables|Default|GetTimeRunner)))
  (Transformation|SetActorLocation _output_get_2 false false))

(event EventBeginPlay
  (Variables|Default|SetSavedLifeTime (Variables|Default|GetLifeTime))
  (Variables|Default|SetSavedHideTime (Variables|Default|GetHideTime))
  (if (Variables|Default|GetIsHideBlock)
    (Rendering|Material|SetMaterial (Variables|Default|GetPlane) 0 "/Game/PaperJack/Materials/Leaf_Ready_Mat.Leaf_Ready_Mat")))

(event EventTick
  (params (DeltaSeconds :type Float%20%28single-precision%29))
  (if (Variables|Default|GetIsLeftRightBlock)
    (CallFunction|LeftRightMovemnet DeltaSeconds)
    (elif (Variables|Default|GetIsUpDownBlock)
      (CallFunction|UpDownMovement DeltaSeconds)))
  (if (Variables|Default|GetIsHideBlock)
    (if (Variables|Default|GetIsStart)
      (bind _output_get (Variables|Default|SetLifeTime (- (Variables|Default|GetLifeTime) DeltaSeconds)))
      (if (<= _output_get (Variables|Default|GetSecondHideSpriteTime))
        (Rendering|Material|SetMaterial (Variables|Default|GetPlane) 0 "/Game/PaperJack/Materials/Leaf_Ready_Mat.Leaf_Ready_Mat")
        (if (<= (Variables|Default|GetLifeTime) 0.0)
          (CallFunction|Hide DeltaSeconds)
          (Rendering|Material|SetMaterial (Variables|Default|GetPlane) 0 "/Game/PaperJack/Materials/Leaf_Hider_Mat.Leaf_Hider_Mat"))
        (else
          (Rendering|Material|SetMaterial (Variables|Default|GetPlane) 0 "/Game/PaperJack/Materials/Leaf_Hider_Mat.Leaf_Hider_Mat"))))
    (else
      (Rendering|Material|SetMaterial (Variables|Default|GetPlane) 0 "/Game/PaperJack/Materials/M_Leaf.M_Leaf"))))

(fn ConstructionScript
  (if (Variables|Default|GetIsHideBlock)
    (Rendering|Material|SetMaterial (Variables|Default|GetPlane) 0 "/Game/PaperJack/Materials/Leaf_Hider_Mat.Leaf_Hider_Mat")
    (else
      (Rendering|Material|SetMaterial (Variables|Default|GetPlane) 0 "/Game/PaperJack/Materials/M_Leaf.M_Leaf"))))