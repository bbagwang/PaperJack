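; Climbable zone, such as a ladder, that lets the PaperJack player move vertically while inside its Box trigger.
; Entering the Box sets CanClimb, stops the character and switches it to Flying, while the Upstair component drops to physics-only collision.
; Leaving restores Walking and query-only collision on Upstair, then nudges the player along its capsule's vertical axis by PushValue.
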(event OnComponentBeginOverlap(Box)
  (params (OverlappedComponent :type Primitive%20Component%20Object%20Reference) (OtherActor :type Actor%20Object%20Reference) (OtherComp :type Primitive%20Component%20Object%20Reference) (OtherBodyIndex :type Integer) (bFromSweep :type Boolean) (SweepResult :type Hit%20Result%20Structure%20%28by%20ref%29))
  (bind _aspaper_jack (Utilities|Casting|CastToPaperJack OtherActor))
  (Variables|/Game/PaperJack/Blueprints/PaperJack.PaperJack_C|SetCanClimb _aspaper_jack true)
  (Components|Movement|StopMovementImmediately (Variables|/Script/Engine.Character|GetCharacterMovement _aspaper_jack))
  (Pawn|Components|CharacterMovement|SetMovementMode (Variables|/Script/Engine.Character|GetCharacterMovement _aspaper_jack) "MOVE_Flying" 0)
  (Collision|SetCollisionEnabled (Variables|Default|GetUpstair) "PhysicsOnly"))

(event OnComponentEndOverlap(Box)
  (params (OverlappedComponent :type Primitive%20Component%20Object%20Reference) (OtherActor :type Actor%20Object%20Reference) (OtherComp :type Primitive%20Component%20Object%20Reference) (OtherBodyIndex :type Integer))
  (bind _player (Variables|Default|GetPlayer))
  (bind _returnvalue (Transformation|GetActorLocation _player))
  (bind _aspaper_jack (Utilities|Casting|CastToPaperJack OtherActor))
  (Variables|/Game/PaperJack/Blueprints/PaperJack.PaperJack_C|SetCanClimb _aspaper_jack false)
  (Pawn|Components|CharacterMovement|SetMovementMode (Variables|/Script/Engine.Character|GetCharacterMovement _aspaper_jack) "MOVE_Walking" 0)
  (Collision|SetCollisionEnabled (Variables|Default|GetUpstair) "QueryOnly")
  (Transformation|SetActorLocation (Variables|Default|GetPlayer) (Math|Vector|MakeVector (.x _returnvalue) (.y _returnvalue) (+ (.z _returnvalue) (* (Variables|Default|GetPushValue) (.z (Math|Vector|GetUpVector (Variables|/Script/Engine.Character|GetCapsuleComponent (Variables|Default|GetPlayer))))))) false false))

(event EventTick
  (params (DeltaSeconds :type Float%20%28single-precision%29)))

(event EventBeginPlay
  (bind _aspaper_jack (Utilities|Casting|CastToPaperJack (Game|Player|GetPlayerPawn 0)))
  (Variables|Default|SetPlayer _aspaper_jack)
  (Variables|Default|SetClimbJumpTimerSave (Variables|Default|GetClimbJumpTimer)))

(fn ConstructionScript)